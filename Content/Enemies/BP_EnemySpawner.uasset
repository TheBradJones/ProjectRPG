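; Combat-zone enemy spawner that starts a wave of AI_EnemyBase when the player enters its Box, which it then moves to world origin.
; WaveSpawner loops delayed spawns at random Arrow transforms up to EnemiesPerWave, with a cooldown and counter reset once none remain.
; Box overlap queries drive these checks and a per-Tick "Enemies Left" text.
; Player exit halts spawning and deals heavy damage to enemies inside.
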(event OnComponentBeginOverlap(Box)
  (params (OverlappedComponent :type Primitive%20Component%20Object%20Reference) (OtherActor :type Actor%20Object%20Reference) (OtherComp :type Primitive%20Component%20Object%20Reference) (OtherBodyIndex :type Integer) (bFromSweep :type Boolean) (SweepResult :type Hit%20Result%20Structure%20%28by%20ref%29))
  (Utilities|Casting|CastToBP_ThirdPersonCharacter OtherActor)
  (Development|PrintString "Hello")
  (CallFunction|WaveSpawner)
  (Variables|Default|SetInsideCombatZone? true)
  (Transformation|SetWorldLocation (Variables|Default|GetBox) "0, 0, 0" false false))

(event OnComponentEndOverlap(Box)
  (params (OverlappedComponent :type Primitive%20Component%20Object%20Reference) (OtherActor :type Actor%20Object%20Reference) (OtherComp :type Primitive%20Component%20Object%20Reference) (OtherBodyIndex :type Integer))
  ;[1 1 1] Stop Spawning Enemies
  (Utilities|Casting|CastToBP_ThirdPersonCharacter OtherActor)
  (Variables|Default|SetInsideCombatZone? false)
  (for _array_element (Collision|GetOverlappingActors (Variables|Default|GetBox) "/Game/Enemies/AI_EnemyBase.AI_EnemyBase_C" :!class /Script/Engine.PrimitiveComponent)
    (bind _asai_enemy_base (Utilities|Casting|CastToAI_EnemyBase _array_element))
    (Default|DamageEnemy _asai_enemy_base 1e+02 true)))

(event Custom|WaveSpawner
  (bind _returnvalue (Math|Random|RandomIntegerinRange 0 6))
  (bind _arrow (Variables|Default|GetArrow))
  (bind _box (Variables|Default|GetBox))
  (bind _arrow1 (Variables|Default|GetArrow1))
  (bind _arrow2 (Variables|Default|GetArrow2))
  (bind _arrow3 (Variables|Default|GetArrow3))
  (bind _arrow4 (Variables|Default|GetArrow4))
  (bind _arrow5 (Variables|Default|GetArrow5))
  (bind _arrow6 (Variables|Default|GetArrow6))
  (bind _overlappingactors (Collision|GetOverlappingActors _box "/Game/Enemies/AI_EnemyBase.AI_EnemyBase_C" :!class /Script/Engine.PrimitiveComponent))
  (bind _returnvalue_2 (Utilities|Select :Index _returnvalue :Option%200 _arrow :Option%201 _arrow1 :Option%202 _arrow2 :Option%203 _arrow3 :Option%204 _arrow4 :Option%205 _arrow5 :Option%206 _arrow6))
  (bind _returnvalue_3 (Utilities|Array|Length _overlappingactors))
  (bind _returnvalue_4 (Transformation|GetWorldTransform _returnvalue_2))
  (bind _returnvalue_5 (== _returnvalue_3 0))
  (if _returnvalue_5
    (Variables|Default|SetNoEnemies true)
    (Utilities|FlowControl|Delay 3.0)
    (if (== (Variables|WaveControl|GetEnemies) (Variables|WaveControl|GetEnemiesPerWave)) :!label _label
      (while (not _returnvalue_5)
        (CallFunction|WaveSpawner))
      (Development|PrintString "All Enemies Killed")
      (Utilities|FlowControl|Delay (Variables|WaveControl|GetWaveCooldown))
      (Development|PrintString "Next Wave")
      (Variables|WaveControl|SetEnemies 0)
      (elif (Variables|Default|GetInsideCombatZone?)
        (Utilities|FlowControl|Delay (Variables|WaveControl|GetSpawnRate))
        (Game|SpawnActorfromClass "/Game/Enemies/AI_EnemyBase.AI_EnemyBase_C" (Math|Transform|MakeTransform (.location _returnvalue_4) (.rotation _returnvalue_4) "1.000000,1.000000,1.000000") "Undefined" "MultiplyWithRoot" 0 "NewEnumerator4" 0)
        (Math|Integer|IncrementInt (Variables|WaveControl|GetEnemies)
          (:%20%20
            (goto _label)))))
    (else
      (Variables|Default|SetNoEnemies false))))

(event EventBeginPlay)

(event EventTick
  (params (DeltaSeconds :type Float%20%28single-precision%29))
  (Rendering|Components|TextRender|SetText (Variables|Default|GetTextRender) (Utilities|Text|FormatText "Enemies Left: {num}" (Utilities|Array|Length (Collision|GetOverlappingActors (Variables|Default|GetBox) "/Game/Enemies/AI_EnemyBase.AI_EnemyBase_C" :!class /Script/Engine.PrimitiveComponent)))))

(fn ConstructionScript)