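; BP_Freeze is a heavy-spell freeze effect that temporarily slows AI_EnemyBase enemies entering its box to a near standstill.
; It reads the effect duration from the level's BP_HeavySpellManager on BeginPlay.
; Each enemy overlap cuts walk speed and destroys the box after a short delay.
; The same event gathers the box's overlapping actors and, after the duration, resets enemy walk speed to a hard-coded value.
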(event OnComponentBeginOverlap(Box)
  (params (OverlappedComponent :type Primitive%20Component%20Object%20Reference) (OtherActor :type Actor%20Object%20Reference) (OtherComp :type Primitive%20Component%20Object%20Reference) (OtherBodyIndex :type Integer) (bFromSweep :type Boolean) (SweepResult :type Hit%20Result%20Structure%20%28by%20ref%29))
  (bind _asai_enemy_base (Utilities|Casting|CastToAI_EnemyBase OtherActor))
  (Utilities|FlowControl|Sequence
    (:then_0
      (Variables|/Script/Engine.CharacterMovementComponent|SetMaxWalkSpeed (Variables|/Script/Engine.Character|GetCharacterMovement _asai_enemy_base) 5.0)
      (Utilities|FlowControl|Delay 0.5)
      (Components|DestroyComponent (Variables|Default|GetBox)))
    (:then_1
      (bind _output_get (Variables|Default|SetOverlapping%20Actors (Collision|GetOverlappingActors (Variables|Default|GetBox) 0 :!class /Script/Engine.PrimitiveComponent)))
      (Utilities|FlowControl|Delay (Variables|Default|GetEffectDuration))
      (for _array_element _output_get
        (bind _asai_enemy_base_2 (Utilities|Casting|CastToAI_EnemyBase _array_element))
        (Variables|/Script/Engine.CharacterMovementComponent|SetMaxWalkSpeed (Variables|/Script/Engine.Character|GetCharacterMovement _asai_enemy_base_2) 3.5e+02)))))

(event EventBeginPlay
  (Utilities|FlowControl|Sequence
    (:then_0
      (bind _outactors (Actor|GetAllActorsOfClass "/Game/Spellcasting/HeavySpells/BP_HeavySpellManager.BP_HeavySpellManager_C"))
      (bind _output_get (Variables|Default|SetBP_HeavySpell (Utilities|Array|Get(acopy) _outactors)))
      (Variables|Default|SetEffectDuration (Variables|/Game/Spellcasting/HeavySpells/BP_HeavySpellManager.BP_HeavySpellManager_C|GetEffectDuration _output_get)))))

(fn ConstructionScript)