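; BP_BasicBlast is a heavy-spell blast that damages target dummies and third-person characters overlapping its sphere.
; On BeginPlay it copies its Damage value from the first BP_HeavySpellManager in the level.
; Sphere overlap starts an undelayed while loop that repeatedly applies that damage, flagged as heavy for players.
; The loop runs on a Looping flag, cleared on end overlap or when another actor type begins overlapping.
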(event OnComponentEndOverlap(Sphere)
  (params (OverlappedComponent :type Primitive%20Component%20Object%20Reference) (OtherActor :type Actor%20Object%20Reference) (OtherComp :type Primitive%20Component%20Object%20Reference) (OtherBodyIndex :type Integer))
  (Variables|Default|SetLooping? false))

(event OnComponentBeginOverlap(Sphere)
  (params (OverlappedComponent :type Primitive%20Component%20Object%20Reference) (OtherActor :type Actor%20Object%20Reference) (OtherComp :type Primitive%20Component%20Object%20Reference) (OtherBodyIndex :type Integer) (bFromSweep :type Boolean) (SweepResult :type Hit%20Result%20Structure%20%28by%20ref%29))
  (bind _damage (Variables|SpellInfo|GetDamage))
  (Variables|Default|SetLooping? true)
  (bind _asbp_target_dummy (Utilities|Casting|CastToBP_TargetDummy OtherActor)
    (:then
      (while (Variables|Default|GetLooping?)
        (Default|DamagetheDummy _asbp_target_dummy _damage)))
    (:CastFailed
      (bind _asbp_third_person_character (Utilities|Casting|CastToBP_ThirdPersonCharacter OtherActor)
        (:then
          (while (Variables|Default|GetLooping?)
            (Default|DamagePlayer _asbp_third_person_character _damage true)))
        (:CastFailed
          (Variables|Default|SetLooping? false))))))

(event EventBeginPlay
  (bind _outactors (Actor|GetAllActorsOfClass "/Game/Spellcasting/HeavySpells/BP_HeavySpellManager.BP_HeavySpellManager_C"))
  (Variables|SpellInfo|SetDamage (Variables|/Game/Spellcasting/HeavySpells/BP_HeavySpellManager.BP_HeavySpellManager_C|GetDamage (Utilities|Array|Get(acopy) _outactors))))

(fn ConstructionScript)