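; Light (non-heavy) spell actor that takes on the player's selected element and deals damage on overlap.
; Tick checks the element through chained branches with DoOnce gates, setting damage, spell cost, sphere material and light color on change.
; Sphere overlap damages the player if the owner's display name contains AI_EnemyBase, otherwise target dummies or enemies.
; Enemy-owned instances also follow the player's element, since Tick always reads player 0.
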(event OnComponentBeginOverlap(Sphere)
  (params (OverlappedComponent :type Primitive%20Component%20Object%20Reference) (OtherActor :type Actor%20Object%20Reference) (OtherComp :type Primitive%20Component%20Object%20Reference) (OtherBodyIndex :type Integer) (bFromSweep :type Boolean) (SweepResult :type Hit%20Result%20Structure%20%28by%20ref%29))
  (if (Utilities|String|Contains (Utilities|GetDisplayName (Components|GetOwner self)) "AI_EnemyBase") ; Did it come from an enemy?
    (bind _asbp_third_person_character (Utilities|Casting|CastToBP_ThirdPersonCharacter OtherActor))
    (Default|DamagePlayer _asbp_third_person_character (Variables|SpellInfo|GetDamage) false)
    (else
      (bind _asbp_target_dummy (Utilities|Casting|CastToBP_TargetDummy OtherActor)
        (:then
          (Default|DamagetheDummy _asbp_target_dummy (Variables|SpellInfo|GetDamage)))
        (:CastFailed
          (bind _asai_enemy_base (Utilities|Casting|CastToAI_EnemyBase OtherActor))
          (Default|DamageEnemy _asai_enemy_base (Variables|SpellInfo|GetDamage) false))))))

(event EventTick
  (params (DeltaSeconds :type Float%20%28single-precision%29))
  (bind _asbp_third_person_character (Utilities|Casting|CastToBP_ThirdPersonCharacter (Game|GetPlayerCharacter 0)))
  (if (Utilities|Enum|Equal(Enum) (Utilities|Struct|BreakStruct_SpellElement (Variables|/Game/ThirdPerson/Blueprints/BP_ThirdPersonCharacter.BP_ThirdPersonCharacter_C|GetSelectedElement _asbp_third_person_character)) "NewEnumerator6")
    (Utilities|FlowControl|DoOnce false :!label _label
      (:Completed
        (Variables|SpellInfo|SetDamage 1.0)
        (Variables|SpellInfo|SetSpellcost 5.0)
        (Rendering|Material|SetMaterial (Variables|Default|GetSphere) 0 "/Game/Materials/LightSpells/M_BasicSpell.M_BasicSpell")
        (Rendering|Components|Light|SetLightColor (Variables|Default|GetPointLight) "(R=0.000000,G=1.000000,B=0.917171,A=1.000000)" true)))
    (else
      (Utilities|FlowControl|Sequence
        (:then_0
          (goto _label Reset))
        (:then_1
          (if (Utilities|Enum|Equal(Enum) (Utilities|Struct|BreakStruct_SpellElement (Variables|/Game/ThirdPerson/Blueprints/BP_ThirdPersonCharacter.BP_ThirdPersonCharacter_C|GetSelectedElement _asbp_third_person_character)) "NewEnumerator0")
            (Utilities|FlowControl|DoOnce false :!label _label_2
              (:Completed
                (Variables|SpellInfo|SetDamage 2.0)
                (Variables|SpellInfo|SetSpellcost 1e+01)
                (Rendering|Material|SetMaterial (Variables|Default|GetSphere) 0 "/Game/Materials/LightSpells/M_FireSpell.M_FireSpell")
                (Rendering|Components|Light|SetLightColor (Variables|Default|GetPointLight) "(R=0.843750,G=0.000000,B=0.000000,A=1.000000)" true)))
            (else
              (Utilities|FlowControl|Sequence
                (:then_0
                  (goto _label_2 Reset))
                (:then_1
                  (if (Utilities|Enum|Equal(Enum) (Utilities|Struct|BreakStruct_SpellElement (Variables|/Game/ThirdPerson/Blueprints/BP_ThirdPersonCharacter.BP_ThirdPersonCharacter_C|GetSelectedElement _asbp_third_person_character)) "NewEnumerator1")
                    (Utilities|FlowControl|DoOnce false :!label _label_3
                      (:Completed
                        (Variables|SpellInfo|SetDamage 2.0)
                        (Variables|SpellInfo|SetSpellcost 1e+01)
                        (Rendering|Material|SetMaterial (Variables|Default|GetSphere) 0 "/Game/Materials/LightSpells/M_IceSpell.M_IceSpell")
                        (Rendering|Components|Light|SetLightColor (Variables|Default|GetPointLight) "(R=0.000000,G=0.097549,B=1.000000,A=1.000000)" true)))
                    (else
                      (Utilities|FlowControl|Sequence
                        (:then_0
                          (goto _label_3 Reset))
                        (:then_1
                          (if (Utilities|Enum|Equal(Enum) (Utilities|Struct|BreakStruct_SpellElement (Variables|/Game/ThirdPerson/Blueprints/BP_ThirdPersonCharacter.BP_ThirdPersonCharacter_C|GetSelectedElement _asbp_third_person_character)) "NewEnumerator3")
                            (Utilities|FlowControl|DoOnce false :!label _label_4
                              (:Completed
                                (Variables|SpellInfo|SetDamage 5.0)
                                (Variables|SpellInfo|SetSpellcost 15.0)
                                (Rendering|Material|SetMaterial (Variables|Default|GetSphere) 0 "/Game/Materials/LightSpells/M_LightningSpell.M_LightningSpell")
                                (Rendering|Components|Light|SetLightColor (Variables|Default|GetPointLight) "(R=1.000000,G=1.000000,B=0.000000,A=1.000000)" true)))
                            (else
                              (Utilities|FlowControl|Sequence
                                (:then_0
                                  (goto _label_4 Reset))
                                (:then_1
                                  (if (Utilities|Enum|Equal(Enum) (Utilities|Struct|BreakStruct_SpellElement (Variables|/Game/ThirdPerson/Blueprints/BP_ThirdPersonCharacter.BP_ThirdPersonCharacter_C|GetSelectedElement _asbp_third_person_character)) "NewEnumerator2")
                                    (Utilities|FlowControl|DoOnce false :!label _label_5
                                      (:Completed
                                        (Variables|SpellInfo|SetDamage 5.0)
                                        (Variables|SpellInfo|SetSpellcost 15.0)
                                        (Rendering|Material|SetMaterial (Variables|Default|GetSphere) 0 "/Game/Materials/LightSpells/M_EarthSpell.M_EarthSpell")
                                        (Rendering|Components|Light|SetLightColor (Variables|Default|GetPointLight) "(R=0.000000,G=0.432000,B=0.000000,A=1.000000)" true)))
                                    (else
                                      (Utilities|FlowControl|Sequence
                                        (:then_0
                                          (goto _label_5 Reset))
                                        (:then_1
                                          (if (Utilities|Enum|Equal(Enum) (Utilities|Struct|BreakStruct_SpellElement (Variables|/Game/ThirdPerson/Blueprints/BP_ThirdPersonCharacter.BP_ThirdPersonCharacter_C|GetSelectedElement _asbp_third_person_character)) "NewEnumerator4")
                                            (Utilities|FlowControl|DoOnce false :!label _label_6
                                              (:Completed
                                                (Variables|SpellInfo|SetDamage 1e+01)
                                                (Variables|SpellInfo|SetSpellcost 2e+01)
                                                (Rendering|Material|SetMaterial (Variables|Default|GetSphere) 0 "/Game/Materials/LightSpells/M_LightSpell.M_LightSpell")
                                                (Rendering|Components|Light|SetLightColor (Variables|Default|GetPointLight) "(R=1.000000,G=1.000000,B=1.000000,A=1.000000)" true)))
                                            (else
                                              (Utilities|FlowControl|Sequence
                                                (:then_0
                                                  (goto _label_6 Reset))
                                                (:then_1
                                                  (if (Utilities|Enum|Equal(Enum) (Utilities|Struct|BreakStruct_SpellElement (Variables|/Game/ThirdPerson/Blueprints/BP_ThirdPersonCharacter.BP_ThirdPersonCharacter_C|GetSelectedElement _asbp_third_person_character)) "NewEnumerator5")
                                                    (Utilities|FlowControl|DoOnce false :!label _label_7
                                                      (:Completed
                                                        (Variables|SpellInfo|SetDamage 1e+01)
                                                        (Variables|SpellInfo|SetSpellcost 2e+01)
                                                        (Rendering|Material|SetMaterial (Variables|Default|GetSphere) 0 "/Game/Materials/LightSpells/M_DarkSpell.M_DarkSpell")
                                                        (Rendering|Components|Light|SetLightColor (Variables|Default|GetPointLight) "(R=0.105977,G=0.000000,B=0.614583,A=1.000000)" true)))
                                                    (else
                                                      (goto _label_7 Reset))))))))))))))))))))))))))))

(fn ConstructionScript)