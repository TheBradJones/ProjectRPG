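; BP_TargetDummy is a target dummy that displays a damage-per-second readout on a TextRender component.
; Its DamageTheDummy event adds incoming damage to a running total and shows that total as text.
; Two parallel Delays on a Sequence zero the total and, later, blank the text, timed from the first hit because further hits do not restart a pending Delay.
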(event Custom|DamageTheDummy
  (params (Damage :type Float%20%28double-precision%29))
  (bind _textrender (Variables|Default|GetTextRender))
  (Utilities|FlowControl|Sequence
    (:then_0
      (bind _output_get (Variables|Default|SetDamagePerSecond (+ Damage (Variables|Default|GetDamagePerSecond))))
      (Rendering|Components|TextRender|SetText _textrender (Utilities|Text|ToText(Float) _output_get "HalfToEven"))
      (Utilities|FlowControl|Delay 2.0)
      (Rendering|Components|TextRender|SetText _textrender (Utilities|Text|MakeLiteralText "")) ; hide dps
    )
    (:then_1
      (Utilities|FlowControl|Delay 1.0)
      (Variables|Default|SetDamagePerSecond 0.0))))

(fn ConstructionScript)